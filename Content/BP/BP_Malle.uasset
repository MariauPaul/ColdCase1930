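; BP_Malle is an examinable trunk (malle) with a code-lock puzzle.
; Examine toggles between a blended camera view showing the WB_Lock widget with mouse cursor, and the player's view.
; On leaving, a solved widget marks the trunk solved, plays its animation and makes DoorRef interactable.
; Examining the solved trunk then fires GettingLight once and hides the Light component, as if picked up.
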(event `self.ReceiveBeginPlay`
  ; set up du widget
  (bind _returnvalue (`|CreateWidget` "/Game/Widget/WB_Lock.WB_Lock_C"))
  (set `self.Widget_ref` _returnvalue))

(event `/Game/BP/BPI/BPI_Lighting_object.Examine`
  (bind _as_bp_third_person_character_1 (`self.As BP Third Person Character_1`))
  ; ouverture du wigdet de code quand interagi avec
  (if (not (`self.Is_Solved`))
    (bind _asbp_third_person_character (cast `/Game/ThirdPerson/Blueprints/BP_ThirdPersonCharacter` (`GameplayStatics.GetPlayerCharacter` 0)))
    (set `self.As BP Third Person Character_1` _asbp_third_person_character)
    (if (not (`/Game/ThirdPerson/Blueprints/BP_ThirdPersonCharacter.Is_Looking` (`self.As BP Third Person Character_1`)))
      (set `/Game/ThirdPerson/Blueprints/BP_ThirdPersonCharacter.Is_Looking` true _as_bp_third_person_character_1)
      (`PlayerController.SetViewTargetWithBlend` (`GameplayStatics.GetPlayerController` 0) (`self.Camera_Ref`) 0.5 "VTBlend_Linear" 0.0 false)
      (`KismetSystemLibrary.Delay` 0.5)
      (`UserWidget.AddToViewport` (`self.Widget_ref`) 0)
      (set `PlayerController.bShowMouseCursor` true (`GameplayStatics.GetPlayerController` 0))
      (else
        (set `/Game/ThirdPerson/Blueprints/BP_ThirdPersonCharacter.Is_Looking` false _as_bp_third_person_character_1)
        (`PlayerController.SetViewTargetWithBlend` (`GameplayStatics.GetPlayerController` 0) (`GameplayStatics.GetPlayerCharacter` 0) 0.5 "VTBlend_Linear" 0.0 false)
        (`Widget.RemoveFromParent` (`self.Widget_ref`))
        (set `PlayerController.bShowMouseCursor` false (`GameplayStatics.GetPlayerController` 0))
        (if (`/Game/Widget/WB_Lock.Is_Solved` (`self.Widget_ref`))
          (set `self.Is_Solved` true)
          (`SkeletalMeshComponent.PlayAnimation` (`self.anim_malle`) "/Game/Meshes/Props/malle/anim_malle/anim_malle_Anim.anim_malle_Anim" false)
          (set `/Game/BP/Bp_Door.Can_interact` true (`self.Door_Ref`)))))
    (else
      (`/Engine/EditorBlueprintResources/StandardMacros.DoOnce` false
        (:`Completed`
          (`self.Getting_Light`)
          (`SceneComponent.SetVisibility` (`self.Light`) false false))))))

(fn `UserConstructionScript`)