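; Gramophone sound actor that plays music continuously in the level by picking tracks at random.
; On BeginPlay it sets the Music audio component to a random entry from the first two sounds in AudioArray and plays it.
; Tick polls whether Music is still playing and starts another random pick when it stops, so the same track can repeat.
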(event `self.ReceiveBeginPlay`
  ;[0.04337 0.052 0.15 0.5] Play Sound Randomly
  (`self.PlayMusic`))

(event `PlayMusic`
  ;[0.04337 0.052 0.15 0.5] Play Sound Randomly
  (`AudioComponent.SetSound` (`self.Music`) (`|GetArrayItem` (`self.AudioArray`) (`KismetMathLibrary.RandomIntegerInRange` 0 1)))
  (`AudioComponent.Play` (`self.Music`) 0.0))

(event `self.ReceiveTick`
  (params (DeltaSeconds :type "Float (single-precision)"))
  ;[0.04337 0.052 0.15 0.5] Play Sound Randomly
  (if (not (`AudioComponent.IsPlaying` (`self.Music`)))
    (`self.PlayMusic`)))

(fn `UserConstructionScript`)