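; Door Blueprint with a code lock puzzle, where examining it toggles a close-up view with an on-screen lock widget.
; BeginPlay creates the lock and end widgets, and Examine blends the view to a referenced camera, shows the lock and cursor, and flags the player as looking.
; A second Examine restores the player view and copies the lock's solved state.
; Once the door is solved, examining it shows the end widget instead.
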(event `self.ReceiveBeginPlay`
  ; set up du widget
  (bind _returnvalue (`|CreateWidget` "/Game/Widget/WB_Lock.WB_Lock_C"))
  (set `self.Widget_Lock_ref` _returnvalue)
  (bind _returnvalue_2 (`|CreateWidget` "/Game/Widget/WB_Fin.WB_Fin_C"))
  (set `self.Widget_Fin_ref` _returnvalue_2))

(event `/Game/BP/BPI/BPI_Lighting_object.Examine`
  (bind _as_bp_third_person_character (`self.As BP Third Person Character`))
  ; ouverture du wigdet de code quand interagi avec
  (if (`self.Can_interact`)
    (if (not (`self.Is_Solved`))
      (bind _asbp_third_person_character (cast `/Game/ThirdPerson/Blueprints/BP_ThirdPersonCharacter` (`GameplayStatics.GetPlayerCharacter` 0)))
      (set `self.As BP Third Person Character` _asbp_third_person_character)
      (if (not (`/Game/ThirdPerson/Blueprints/BP_ThirdPersonCharacter.Is_Looking` (`self.As BP Third Person Character`)))
        (set `/Game/ThirdPerson/Blueprints/BP_ThirdPersonCharacter.Is_Looking` true _as_bp_third_person_character)
        (`PlayerController.SetViewTargetWithBlend` (`GameplayStatics.GetPlayerController` 0) (`self.Camera_Ref`) 0.5 "VTBlend_Linear" 0.0 false)
        (`KismetSystemLibrary.Delay` 0.5)
        (`UserWidget.AddToViewport` (`self.Widget_Lock_ref`) 0)
        (set `PlayerController.bShowMouseCursor` true (`GameplayStatics.GetPlayerController` 0))
        (else
          (set `/Game/ThirdPerson/Blueprints/BP_ThirdPersonCharacter.Is_Looking` false _as_bp_third_person_character)
          (`PlayerController.SetViewTargetWithBlend` (`GameplayStatics.GetPlayerController` 0) (`GameplayStatics.GetPlayerCharacter` 0) 0.5 "VTBlend_Linear" 0.0 false)
          (`Widget.RemoveFromParent` (`self.Widget_Lock_ref`))
          (set `PlayerController.bShowMouseCursor` false (`GameplayStatics.GetPlayerController` 0))
          (if (`/Game/Widget/WB_Lock.Is_Solved` (`self.Widget_Lock_ref`))
            (set `self.Is_Solved` true))))
      (else
        (`UserWidget.AddToViewport` (`self.Widget_Fin_ref`) 0)))))

(fn `UserConstructionScript`)