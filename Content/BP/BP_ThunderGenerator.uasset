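; BP_ThunderGenerator creates recurring random thunderstorm effects, pairing thunder playback with flashes of a directional light.
; Each cycle picks one of three thunder components and uses the same random index to select a timeline curve that drives light intensity.
; When the timeline finishes, it restores the intensity saved at BeginPlay, waits a random delay and calls itself to repeat indefinitely.
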(event `self.ReceiveBeginPlay`
  (set `self.ThunderArray` (`|MakeArray` (`self.Thundr3`) (`self.Thundr2`) (`self.Thundr1`)))
  (set `self.Intensity` (`LightComponentBase.Intensity` (`self.DirectionalLight`)))
  (`self.LoopRandomThunder`))

(event `LoopRandomThunder`
  (set `self.RandomValue` (`KismetMathLibrary.RandomFloatInRange` 30.0 60.0))
  (set `self.RandomInt` (`KismetMathLibrary.RandomIntegerInRange` 0 2))
  (`AudioComponent.Play` (`|GetArrayItem` (`self.ThunderArray`) (`self.RandomInt`)) 0.0)
  (bind (_direction _1stpatern _2ndpatern _3rdpatern) (`Timeline|LightPatern` :!via `PlayFromStart`)
    (:`Update`
      (bind _output_get (set `self.PaternArray` (`|MakeArray` _1stpatern _2ndpatern _3rdpatern :!type "Float (double-precision)")))
      (`LightComponent.SetIntensity` (`self.DirectionalLight`) (* (`|GetArrayItem` _output_get (`self.RandomInt`)) 1000.0)))
    (:`Finished`
      (`LightComponent.SetIntensity` (`self.DirectionalLight`) (`self.Intensity`))
      (`KismetSystemLibrary.Delay` (`self.RandomValue`))
      (`self.LoopRandomThunder`))))

(fn `UserConstructionScript`)