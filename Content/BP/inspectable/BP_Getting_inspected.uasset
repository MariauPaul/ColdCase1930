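; Temporary inspection actor that shows an item mesh through a scene capture, alongside a WB_inspect widget with its name and description.
; Inspection moves input from the player to this actor, with setters for the item's starting rotation and scale.
; Left-click-gated mouse axes or move input rotate the item, the wheel zooms via clamped capture FOV, and right-click resets both.
; Interact restores player input, removes the widget and destroys the actor.
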(event `EnhancedInput|/Game/ThirdPerson/Input/Actions/IA_Mouse_Right_Clic`
  (params (ActionValue :type Boolean) (ElapsedSeconds :type "Float (double-precision)") (TriggeredSeconds :type "Float (double-precision)") (InputAction :type "InputAction Object Reference" :default "/Game/ThirdPerson/Input/Actions/IA_Mouse_Right_Clic.IA_Mouse_Right_Clic"))
  ;[1 1 1] reset transform
  (:`Started`
    (`SceneComponent.K2_SetWorldRotation` (`self.Item`) (`self.Initial_Rotation`) false false)
    (set `SceneCaptureComponent2D.FOVAngle` 50.0 (`self.SceneCaptureComponent2D`))))

(event `/Game/BP/BPI/BPI_Lighting_object.Inspection`
  (params (Player_ref :type "/Game/ThirdPerson/Blueprints/BP_ThirdPersonCharacter Object Reference") (Object_ref :type "StaticMesh Object Reference") (`item name` :type Text) (`item description` :type Text))
  (bind _returnvalue (`GameplayStatics.GetPlayerController` 0))
  ;[1 1 1] ouvrir le widget d'inspection
  (set `self.Player Ref` Player_ref)
  (`StaticMeshComponent.SetStaticMesh` (`self.Item`) Object_ref)
  (bind _returnvalue_2 (`|CreateWidget` "/Game/BP/inspectable/WB_inspect.WB_inspect_C" null `item name` `item description`))
  (bind _output_get (set `self.Inspect_Widget_ref` _returnvalue_2))
  (`UserWidget.AddToViewport` _output_get 0)
  (`self.DisableInput` (`self.Player Ref`) _returnvalue)
  (`self.EnableInput` _returnvalue))

(event `InputAxisKey|MouseX`
  (params (AxisValue :type "Float (single-precision)"))
  ;[1 1 1] set mouse mouvement horizontal
  (if (`self.Rotate?`)
    (`SceneComponent.K2_SetWorldRotation` (`self.Item`) (`KismetMathLibrary.ComposeRotators` (`SceneComponent.K2_GetComponentRotation` (`self.Item`)) (`KismetMathLibrary.MakeRotator` 0.0 0.0 (* AxisValue -3.0))) false false)))

(event `EnhancedInput|/Game/ThirdPerson/Input/Actions/IA_Interaction`
  (params (ActionValue :type Boolean) (ElapsedSeconds :type "Float (double-precision)") (TriggeredSeconds :type "Float (double-precision)") (InputAction :type "InputAction Object Reference" :default "/Game/ThirdPerson/Input/Actions/IA_Interaction.IA_Interaction"))
  (bind _returnvalue (`GameplayStatics.GetPlayerController` 0))
  ;[1 1 1] retirer le Wigdet quand il est ouvert
  (:`Started`
    (`self.DisableInput` _returnvalue)
    (`self.EnableInput` (`self.Player Ref`) _returnvalue)
    (`/Engine/EditorBlueprintResources/StandardMacros.IsValid` (`self.Inspect_Widget_ref`)
      (:`Is Valid`
        (`Widget.RemoveFromParent` (`self.Inspect_Widget_ref`))
        (set `self.Inspect_Widget_ref` null)
        (`self.K2_DestroyActor`)))))

(event `InputAxisKey|MouseY`
  (params (AxisValue :type "Float (single-precision)"))
  ;[1 1 1] set mouse mouvement vertical
  (if (`self.Rotate?`)
    (`SceneComponent.K2_SetWorldRotation` (`self.Item`) (`KismetMathLibrary.ComposeRotators` (`SceneComponent.K2_GetComponentRotation` (`self.Item`)) (`KismetMathLibrary.MakeRotator` 0.0 (* AxisValue -3.0))) false false)))

(event `Set inspect rotation`
  (params (Item_rotation :type "Rotator Structure"))
  (bind _item (`self.Item`))
  (bind (_returnvalue_location _returnvalue_rotation _returnvalue_scale) (`KismetMathLibrary.BreakTransform` (`SceneComponent.K2_GetComponentToWorld` _item)))
  ;[1 1 1] Set inspection rotation
  (bind _output_get (set `self.Initial_Rotation` Item_rotation))
  (`SceneComponent.K2_SetWorldTransform` _item (`KismetMathLibrary.MakeTransform` _returnvalue_location _output_get _returnvalue_scale) false false))

(event `Set_Inspect_Scale`
  (params (Inspection_Scale :type "Vector Structure"))
  (bind _item (`self.Item`))
  (bind (_returnvalue_location _returnvalue_rotation) (`KismetMathLibrary.BreakTransform` (`SceneComponent.K2_GetComponentToWorld` _item)))
  ;[1 1 1] set inspection scale
  (`SceneComponent.K2_SetWorldTransform` _item (`KismetMathLibrary.MakeTransform` _returnvalue_location _returnvalue_rotation Inspection_Scale) false false))

(event `EnhancedInput|/Game/ThirdPerson/Input/Actions/IA_Move`
  (params (ActionValue :type "Vector2D Structure") (ElapsedSeconds :type "Float (double-precision)") (TriggeredSeconds :type "Float (double-precision)") (InputAction :type "InputAction Object Reference" :default "/Game/ThirdPerson/Input/Actions/IA_Move.IA_Move"))
  ;[1 1 1] Move with ZQSD
  (:`Triggered`
    (if (or (!= ActionValue_X 0.0) (!= ActionValue_Y 0.0))
      (`|ExecutionSequence`
        (:`then_0`
          (`SceneComponent.K2_SetWorldRotation` (`self.Item`) (`KismetMathLibrary.ComposeRotators` (`SceneComponent.K2_GetComponentRotation` (`self.Item`)) (`KismetMathLibrary.MakeRotator` 0.0 0.0 (* ActionValue_X -2.0))) false false))
        (:`then_1`
          (`SceneComponent.K2_SetWorldRotation` (`self.Item`) (`KismetMathLibrary.ComposeRotators` (`SceneComponent.K2_GetComponentRotation` (`self.Item`)) (`KismetMathLibrary.MakeRotator` 0.0 (* ActionValue_Y -2.0))) false false))))))

(event `EnhancedInput|/Game/ThirdPerson/Input/Actions/IA_Left_Mouse_Clic`
  (params (ActionValue :type Boolean) (ElapsedSeconds :type "Float (double-precision)") (TriggeredSeconds :type "Float (double-precision)") (InputAction :type "InputAction Object Reference" :default "/Game/ThirdPerson/Input/Actions/IA_Left_Mouse_Clic.IA_Left_Mouse_Clic"))
  ;[1 1 1] can rotate only when clic mouse
  (:`Started`
    (set `self.Rotate?` true))
  (:`Ongoing`
    (set `self.Rotate?` false)))

(event `EnhancedInput|/Game/ThirdPerson/Input/Actions/IA_Mouse_Wheel_Up`
  (params (ActionValue :type Boolean) (ElapsedSeconds :type "Float (double-precision)") (TriggeredSeconds :type "Float (double-precision)") (InputAction :type "InputAction Object Reference" :default "/Game/ThirdPerson/Input/Actions/IA_Mouse_Wheel_Up.IA_Mouse_Wheel_Up"))
  (bind _scenecapturecomponent2d (`self.SceneCaptureComponent2D`))
  ;[1 1 1] Zoom in
  (:`Triggered`
    (set `SceneCaptureComponent2D.FOVAngle` (`KismetMathLibrary.FClamp` (- (`SceneCaptureComponent2D.FOVAngle` _scenecapturecomponent2d) 1.0) 30.0 80.0) _scenecapturecomponent2d)))

(event `EnhancedInput|/Game/ThirdPerson/Input/Actions/IA_Mouse_Wheel_Down`
  (params (ActionValue :type Boolean) (ElapsedSeconds :type "Float (double-precision)") (TriggeredSeconds :type "Float (double-precision)") (InputAction :type "InputAction Object Reference" :default "/Game/ThirdPerson/Input/Actions/IA_Mouse_Wheel_Down.IA_Mouse_Wheel_Down"))
  (bind _scenecapturecomponent2d (`self.SceneCaptureComponent2D`))
  ;[1 1 1] Zoom out
  (:`Triggered`
    (set `SceneCaptureComponent2D.FOVAngle` (`KismetMathLibrary.FClamp` (+ (`SceneCaptureComponent2D.FOVAngle` _scenecapturecomponent2d) 1.0) 30.0 80.0) _scenecapturecomponent2d)))

(fn `UserConstructionScript`)